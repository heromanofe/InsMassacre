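; Gas mask gear item that moves its third-person mesh between the carrier's gas mask socket, the weapon bone and the head socket as its equip state changes.
; On pickup it caches head, headgear, facewear and eyewear info from the soldier's cosmetics, preferring the merged mesh.
; Equipping or unequipping toggles gender-specific gasmask morphs on those meshes and hides eyewear material sections on every LOD.
; Preview actors attach to the ammo vest.
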(event Custom|MeshLoaded
  (params (MeshComponent :type INS%20Skeletal%20Mesh%20Component%20Object%20Reference))
  (bind _mesh (CallFunction|GetEquipmentMesh (Variables|Default|GetSoldier)))
  (CallFunction|AttachGasmaskSocket _mesh))

(event Collision|EventActorBeginOverlap
  (params (OtherActor :type Actor%20Object%20Reference)))

(event EventAttachGogglestoComponent
  (params (TargetComponent :type INS%20Skeletal%20Mesh%20Component%20Object%20Reference))
  (CallFunction|AttachGasmaskSocket TargetComponent))

(event EventBlueprintonPickedUp
  (bind _asinssoldier (Utilities|Casting|CastToINSSoldier (Components|GetOwner)))
  (Variables|Default|SetSoldier _asinssoldier)
  (Utilities|FlowControl|Sequence
    (:then_0
      (EventDispatchers|BindEventtoOnMesh3PLoadedDelegate self (delegate Custom|MeshLoaded)))
    (:then_1
      (Cosmetics|GetHeadCosmetic)
      (Cosmetics|UpdateHeadgearEyewear false (Class|INSSoldier|GetSharedCosmeticState (Variables|Default|GetSoldier))))))

(event EventBlueprintSpawnedPreviewActor
  (params (bFirstPerson :type Boolean) (PlayerInventory :type Player%20Inventory%20Component%20Object%20Reference))
  (Cosmetics|SetupPreviewAttachment))

(event EventBlueprintonAttachMeshtoPawn
  (params (Mesh :type INS%20Skeletal%20Mesh%20Component%20Object%20Reference))
  (bind _mesh (CallFunction|GetEquipmentMesh (Variables|Default|GetSoldier)))
  (CallFunction|AttachGasmaskSocket _mesh))

(event EventBlueprintInteractableStateChanged
  (params (NewState :type EEquipableState%20Enum :default "ES_Unequipped"))
  (bind _soldier (Variables|Default|GetSoldier))
  (bind _returnvalue (Class|INSSoldier|GetSharedCosmeticState _soldier))
  (Class|CharacterAnimInterface|UpdateGasMaskState(Message) (Components|SkeletalMesh|GetAnimInstance (Variables|/Script/Engine.Character|GetMesh (Variables|Default|GetSoldier))) NewState)
  (switch Utilities|FlowControl|Switch|SwitchonEEquipableState NewState
    (:ES_Unequipped
      (bind _mesh (CallFunction|GetEquipmentMesh (Variables|Default|GetSoldier)))
      (CallFunction|AttachGasmaskSocket _mesh))
    (:ES_Equipping
      (Transformation|AttachComponentToComponent (Class|ItemBase|GetMesh3P) (Variables|/Script/Engine.Character|GetMesh (Variables|Default|GetSoldier)) "b_wpn" "KeepRelative" "KeepRelative" "KeepRelative" false))
    (:ES_Equipped
      (CallFunction|AttachGasMaskHead)
      (Cosmetics|UpdateHeadgearEyewear true _returnvalue))
    (:ES_Unequipping
      (Cosmetics|UpdateHeadgearEyewear false _returnvalue))))

(fn ConstructionScript
  (Transformation|SetActorRelativeTransform (Math|Transform|MakeTransform "0, 0, 0") false false))

(fn GetHeadCosmetic
  (if (Utilities|Name|Equal(Name) (Variables|Cosmetics|GetHeadMorph) "None")
    (bind _soldier (Variables|Default|GetSoldier)
      (:then
        (bind _returnvalue (Class|INSSoldier|GetMergedMesh _soldier))
        (Utilities|IsValid _returnvalue
          (:Is%20Valid
            (Utilities|IsValid (Class|INSSoldier|GetSharedCosmeticState _soldier)
              (:Is%20Valid
                (Variables|Cosmetics|SetIsFemale (Variables|/Script/Insurgency.SharedCosmeticState|GetbIsFemale (Class|INSSoldier|GetSharedCosmeticState _soldier)))
                (Variables|Cosmetics|SetHeadMorph (Variables|/Script/Insurgency.SharedCosmeticState|GetHeadMorph (Class|INSSoldier|GetSharedCosmeticState _soldier)))
                (Variables|Cosmetics|SetEyewearHeadMorph (Variables|/Script/Insurgency.SharedCosmeticState|GetEyewearHeadMorph (Class|INSSoldier|GetSharedCosmeticState _soldier)))
                (Variables|Cosmetics|SetbFoundEyewear (Variables|/Script/Insurgency.SharedCosmeticState|GetbHasEyewear (Class|INSSoldier|GetSharedCosmeticState _soldier)))
                (Variables|Cosmetics|SetbFoundHeadwear (or (Variables|/Script/Insurgency.SharedCosmeticState|GetbHasHeadgear (Class|INSSoldier|GetSharedCosmeticState _soldier)) (Variables|/Script/Insurgency.SharedCosmeticState|GetbHasFacewear (Class|INSSoldier|GetSharedCosmeticState _soldier)))))))
          (:Is%20Not%20Valid
            ;[1 1 1] Only check for individual cosmetics if merged mesh isn't valid
            (bind _array_element (Utilities|Array|ForEachLoopwithBreak (Variables|/Script/Insurgency.INSSoldier|GetSpawnedCosmetics _soldier))
              (:LoopBody
                (Utilities|IsValid _array_element
                  (:Is%20Valid
                    (bind _ascc_base_head (Utilities|Casting|CastToCC_BASE_HEAD _array_element)
                      (:then
                        (Variables|Cosmetics|SetIsFemale (Variables|/Script/Insurgency.SharedCosmeticState|GetbIsFemale (Variables|/Script/Insurgency.CosmeticItem|GetSharedCosmeticState _ascc_base_head)))
                        (Variables|Cosmetics|SetHeadMorph (Variables|/Script/Insurgency.SharedCosmeticState|GetHeadMorph (Variables|/Script/Insurgency.CosmeticItem|GetSharedCosmeticState _ascc_base_head)))
                        (Variables|Cosmetics|SetEyewearHeadMorph (Variables|/Script/Insurgency.SharedCosmeticState|GetEyewearHeadMorph (Variables|/Script/Insurgency.CosmeticItem|GetSharedCosmeticState _ascc_base_head))))
                      (:CastFailed
                        ;[1 1 1] Check for Headgear and Facewear separately because it's possible to wear both.
                        (if (Utilities|ClassIsChildOf (Utilities|GetClass _array_element) "/Game/Game/Collectibles/Cosmetics/Character/HeadGear/CC_BASE_HDGR.CC_BASE_HDGR_C")
                          (Variables|Cosmetics|SetHeadGearReference (Utilities|Array|Get(acopy) (Variables|/Script/Insurgency.CosmeticItem|GetMesh3PAttachedMeshes _array_element)))
                          (Variables|Cosmetics|SetbFoundHeadwear true :!label _label)
                          (elif (Utilities|ClassIsChildOf (Utilities|GetClass _array_element) "/Game/Game/Collectibles/Cosmetics/Character/FaceWear/CC_BASE_FACEWEAR.CC_BASE_FACEWEAR_C")
                            (Variables|Cosmetics|SetFacewearReference (Utilities|Array|Get(acopy) (Variables|/Script/Insurgency.CosmeticItem|GetMesh3PAttachedMeshes _array_element)))
                            (goto _label)
                            (else
                              ;[0 0.5 1] Check for Eyewear
                              (if (Utilities|ClassIsChildOf (Utilities|GetClass _array_element) "/Game/Game/Collectibles/Cosmetics/Character/Eyewear/CC_BASE_EYE.CC_BASE_EYE_C")
                                (Variables|Cosmetics|SetEyewearReference (Utilities|Array|Get(acopy) (Variables|/Script/Insurgency.CosmeticItem|GetMesh3PAttachedMeshes _array_element)))
                                (Variables|Cosmetics|SetbFoundEyewear true)
                                (elif (Utilities|ClassIsChildOf (Utilities|GetClass _array_element) "/Game/Game/Collectibles/Cosmetics/Character/Hair/CC_BASE_HIJAB.CC_BASE_HIJAB_C")
                                  (Variables|Cosmetics|SetHairReference (Utilities|Array|Get(acopy) (Variables|/Script/Insurgency.CosmeticItem|GetMesh3PAttachedMeshes _array_element)))))))))))))))))
      (:else))))

(fn GetEquipmentMesh
  (params (Soldier :type INS%20Soldier%20Object%20Reference))
  (bind _returnvalue (Class|INSSoldier|GetGearinSlot Soldier "AmmoCarrier"))
  (Utilities|IsValid Soldier
    (:Is%20Valid
      (Utilities|IsValid _returnvalue
        (:Is%20Valid
          (bind _asbp_gear_base_carrier (Utilities|Casting|CastToBP_Gear_BASE_Carrier _returnvalue))
          (return (Class|ItemBase|GetMesh3P _asbp_gear_base_carrier)))))))

(fn AttachGasmaskSocket
  (params (CompositeGear :type INS%20Skeletal%20Mesh%20Component%20Object%20Reference))
  (bind _returnvalue (Class|ItemBase|GetMesh3P))
  (Utilities|IsValid CompositeGear
    (:Is%20Valid
      (Utilities|IsValid _returnvalue
        (:Is%20Valid
          (Utilities|IsValid (Variables|/Script/Engine.SkinnedMeshComponent|GetSkeletalMesh CompositeGear)
            (:Is%20Valid
              (Transformation|AttachComponentToComponent _returnvalue CompositeGear "Equip_Gasmask" "KeepRelative" "KeepRelative" "KeepRelative" false)
              (Transformation|SetActorRelativeTransform (Math|Transform|MakeTransform "0, 0, 0") false false))))))))

(fn AttachGasMaskHead
  (Transformation|AttachComponentToComponent (Class|ItemBase|GetMesh3P) (Variables|/Script/Engine.Character|GetMesh (Variables|Default|GetSoldier)) "s_equip_head_gasmask" "KeepRelative" "KeepRelative" "KeepRelative" false)
  (Cosmetics|GasMaskSetMorph (Class|ItemBase|GetMesh3P))
  (Transformation|SetActorRelativeTransform (Math|Transform|MakeTransform "0, 0, 0") false false))

(fn AttachGasMaskWeapon
  (Transformation|AttachComponentToComponent (Class|ItemBase|GetMesh3P) (Variables|/Script/Engine.Character|GetMesh (Variables|Default|GetSoldier)) "b_wpn" "KeepRelative" "KeepRelative" "KeepRelative" false)
  (Components|SkeletalMesh|SetMorphTarget (Class|ItemBase|GetMesh3P) "HDGR_Unequipped" 0.0 true))

(fn SetupPreviewAttachment
  (bind _returnvalue (Components|GetOwner))
  (Utilities|IsValid _returnvalue
    (:Is%20Valid
      (for _array_element (Actor|GetAttachedActors _returnvalue true)
        (Utilities|IsValid _array_element
          (:Is%20Valid
            (bind _asitem_ammo_vest (Utilities|Casting|CastToItemAmmoVest _array_element))
            (CallFunction|AttachGasmaskSocket (Class|ItemBase|GetMesh3P _asitem_ammo_vest))
            (return))))
      (Transformation|AttachActorToActor (Components|GetOwner) "None" "KeepRelative" "KeepRelative" "KeepRelative" true) ; Just attach to actor, let carrier_none reattach to the proper socket once that is spawned in.
    )))

(fn UpdateHeadgearEyewear
  (params (GasMaskEquipped :type Boolean) (CosmeticState :type Shared%20Cosmetic%20State%20Object%20Reference))
  (bind _isfemale (Variables|Cosmetics|GetIsFemale))
  (bind _returnvalue (Math|Conversions|ToFloat(Boolean) GasMaskEquipped))
  (bind _returnvalue_2 (select _isfemale "_FM" "_ML"))
  (if (Utilities|IsValid CosmeticState)
    (LocalVariables|SetLocalFacewearMorph (Variables|/Script/Insurgency.SharedCosmeticState|GetFacewearMorph CosmeticState))
    (bind _soldier (Variables|Default|GetSoldier)
      (:then
        (bind _returnvalue_3 (Class|INSSoldier|GetMergedMesh _soldier))
        (Utilities|IsValid _returnvalue_3
          (:Is%20Valid
            (Utilities|IsValid (Variables|/Script/Engine.Character|GetMesh _soldier)
              (:Is%20Valid
                ;[1 1 1] Replaces all the cosmetic reference meshes with the merged mesh if it exists.
                (bind _output_get (Variables|Cosmetics|SetMergedMeshReference (Variables|/Script/Engine.Character|GetMesh _soldier)))
                (bind _output_get_2 (Variables|Cosmetics|SetEyewearReference _output_get))
                (bind _output_get_3 (Variables|Cosmetics|SetHeadGearReference _output_get_2))
                (bind _output_get_4 (Variables|Cosmetics|SetFacewearReference _output_get_3))
                (Variables|Cosmetics|SetHairReference _output_get_4))
              (:Is%20Not%20Valid
                _)))
          (:Is%20Not%20Valid
            _)))
      (:else
        _)))
  (if (Variables|Cosmetics|GetbFoundEyewear)
    (Cosmetics|ToggleEyewear (not GasMaskEquipped) (Variables|Cosmetics|GetEyewearReference)))
  (if (Variables|Cosmetics|GetbFoundHeadwear)
    (Utilities|FlowControl|Sequence
      (:then_0
        (bind _headgearreference (Variables|Cosmetics|GetHeadGearReference)
          (:then
            (Components|SkeletalMesh|SetMorphTarget _headgearreference (Utilities|String|StringToName (Utilities|String|Append "HDGR_Gasmask" _returnvalue_2)) _returnvalue true)
            ;[1 1 1] Disables Eyewear Morphs on Headgear
            (if (Variables|Cosmetics|GetbFoundEyewear)
              (Components|SkeletalMesh|SetMorphTarget _headgearreference (Variables|Cosmetics|GetHeadMorph) (Math|Conversions|ToFloat(Boolean) GasMaskEquipped) true)
              (Components|SkeletalMesh|SetMorphTarget _headgearreference (Variables|Cosmetics|GetEyewearHeadMorph) (Math|Conversions|ToFloat(Boolean) (not GasMaskEquipped)) true)))
          (:else)))
      (:then_1
        (bind _hairreference (Variables|Cosmetics|GetHairReference)
          (:then
            (Components|SkeletalMesh|SetMorphTarget _hairreference (Utilities|String|StringToName (Utilities|String|Append "HAIR_Gasmask" _returnvalue_2)) _returnvalue true))
          (:else)))
      (:then_2
        ;[1 1 1] Temporarily disabled because Nik implemented a workaround to have the gasmask further away from the facewear. May need to re enable later
        (bind _facewearreference (Variables|Cosmetics|GetFacewearReference)
          (:then
            (if (or (Utilities|Name|Equal(Name) (LocalVariables|GetLocalFacewearMorph) "Ballistic") (Utilities|Name|Equal(Name) (LocalVariables|GetLocalFacewearMorph) "HalfFace"))
              (Components|SkeletalMesh|SetMorphTarget _facewearreference (Utilities|String|StringToName (Utilities|String|Append "FCWR_Gasmask" _returnvalue_2)) _returnvalue true)))
          (:else)))
      (:then_3
        (bind _mergedmeshreference (Variables|Cosmetics|GetMergedMeshReference)
          (:then
            (Components|SkeletalMesh|SetMorphTarget _mergedmeshreference (Utilities|String|StringToName (Utilities|String|Append "TORSO_Gasmask" _returnvalue_2)) _returnvalue true))
          (:else))))))

(fn ToggleEyewear
  (params (Show :type Boolean) (SkeletalMesh :type Skeletal%20Mesh%20Component%20Object%20Reference))
  (Utilities|IsValid SkeletalMesh
    (:Is%20Valid
      (for _index (range 0 (StaticMesh|GetNumLODs SkeletalMesh))
        (Class|SkinnedMeshComponent|ShowMaterialSection SkeletalMesh (Rendering|Material|GetMaterialIndex SkeletalMesh "Eyewear") 0 Show _index)
        (Class|SkinnedMeshComponent|ShowMaterialSection SkeletalMesh (Rendering|Material|GetMaterialIndex SkeletalMesh "EyewearLens") 0 Show _index)))))

(fn GasMaskSetMorph
  (params (Mesh :type INS%20Skeletal%20Mesh%20Component%20Object%20Reference))
  (if (Utilities|Name|Equal(Name) (Variables|Cosmetics|GetHeadMorph) "None")
    (Cosmetics|GetHeadCosmetic))
  ;[1 0 0] Deprecated Morphs.
  (Components|SkeletalMesh|SetMorphTarget Mesh (Variables|Cosmetics|GetHeadMorph) 1.0 true)
  (Components|SkeletalMesh|SetMorphTarget Mesh "HDGR_Unequipped" 0.0 true))